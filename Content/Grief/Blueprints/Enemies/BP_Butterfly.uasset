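; BP_Butterfly is a flying enemy that constantly follows the player pawn.
; Each tick, after the parent tick, it issues a flight-enabled AI move toward the player's current location with an acceptance radius.
; Movement output updates its facing directions from the movement vector and its moving state, while success or failure updates only the moving state.
; The player sensed and escaped events are empty, so sensing does not gate the chase.
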(event `self.ReceiveTick`
  (params (DeltaSeconds :type "Float (single-precision)"))
  (`parent.ReceiveTick` DeltaSeconds)
  (`AIPawnFunctionLibrary.AIPawnMoveToLocation` (`AIBlueprintHelperLibrary.GetAIController` self) (`self.K2_GetActorLocation` (`GameplayStatics.GetPlayerPawn` 0)) 200.0 true
    (:`Out`
      (`self.UpdateDirections` (`self.GetMovementVector`))
      (`self.UpdateMoving`))
    (:`Success`
      (`self.UpdateMoving`))
    (:`Failure`
      (`self.UpdateMoving`))))

(event `self.PlayerSensing.OnPlayerSensed`
  (params (Player :type "PlayerPawn Object Reference") (Detected :type Boolean) (SensingRange :type "ESensingRange Enum" :default "None") (HasLineOfSight :type Boolean)))

(event `self.PlayerSensing.OnPlayerEscaped`
  (params (Player :type "PlayerPawn Object Reference")))

(fn `UserConstructionScript`)