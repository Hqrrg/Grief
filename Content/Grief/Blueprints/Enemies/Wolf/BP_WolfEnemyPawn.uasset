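; BP_WolfEnemyPawn is the wolf enemy pawn, which feeds player detection into its AI Blackboard to switch chasing on and off.
; It caches its AI controller's Blackboard on BeginPlay.
; When PlayerSensing detects a player, it sets the chase flag and stores the player as a Blackboard object.
; When the player escapes, it clears only the flag and calls UpdateMoving.
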(event `self.ReceiveBeginPlay`
  (set `self.BlackboardRef` (`AIBlueprintHelperLibrary.GetBlackboard` (`AIBlueprintHelperLibrary.GetAIController` self))))

(event `self.PlayerSensing.OnPlayerSensed`
  (params (Player :type "PlayerPawn Object Reference") (Detected :type Boolean) (SensingRange :type "ESensingRange Enum" :default "None") (HasLineOfSight :type Boolean))
  (if Detected
    (`BlackboardComponent.SetValueAsBool` (`self.BlackboardRef`) "InChase?" true)
    (`BlackboardComponent.SetValueAsObject` (`self.BlackboardRef`) "Player" Player)))

(event `self.PlayerSensing.OnPlayerEscaped`
  (params (Player :type "PlayerPawn Object Reference"))
  (`BlackboardComponent.SetValueAsBool` (`self.BlackboardRef`) "InChase?" false)
  (`EnemyPawn.UpdateMoving`))

(fn `UserConstructionScript`)