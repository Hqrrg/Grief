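; BP_Butterfly is a butterfly enemy that passes player detection results to its AI.
; Its PlayerSensing events update the AI controller's blackboard.
; A positive detection sets the "Spotted?" flag and stores the sensed player under "Player".
; An escape clears only the flag, leaving the Player reference in place.
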(event `self.PlayerSensing.OnPlayerSensed`
  (params (Player :type "PlayerPawn Object Reference") (Detected :type Boolean) (SensingRange :type "ESensingRange Enum" :default "None") (HasLineOfSight :type Boolean))
  (bind _returnvalue (`AIBlueprintHelperLibrary.GetBlackboard` (`AIBlueprintHelperLibrary.GetAIController` self)))
  (if Detected
    (`BlackboardComponent.SetValueAsBool` _returnvalue "Spotted?" true)
    (`BlackboardComponent.SetValueAsObject` _returnvalue "Player" Player)))

(event `self.PlayerSensing.OnPlayerEscaped`
  (params (Player :type "PlayerPawn Object Reference"))
  (`BlackboardComponent.SetValueAsBool` (`AIBlueprintHelperLibrary.GetBlackboard` (`AIBlueprintHelperLibrary.GetAIController` self)) "Spotted?" false))

(fn `UserConstructionScript`)