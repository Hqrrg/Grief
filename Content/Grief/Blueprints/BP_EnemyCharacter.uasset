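; BP_EnemyCharacter is an enemy character that chases the player.
; On BeginPlay it caches the player as a BP_PlayerCharacter reference, then every tick issues an AI Move To toward that actor.
; Each tick also updates its facing directions from its movement vector and refreshes its moving state, which is refreshed again when a move succeeds or fails.
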(event `self.ReceiveBeginPlay`
  (bind _asbp_player_character (cast `/Game/Grief/Blueprints/Player/BP_PlayerCharacter` (`GameplayStatics.GetPlayerCharacter` 0)))
  (set `self.PlayerRef` _asbp_player_character))

(event `self.ReceiveTick`
  (params (DeltaSeconds :type "Float (single-precision)"))
  (`|AIMoveTo` self (0.0 0.0 0.0) (`self.PlayerRef`) 100.0
    (:`then`
      (`self.UpdateDirections` (`self.GetMovementVector`))
      (`self.UpdateMoving`))
    (:`OnSuccess`
      (`self.UpdateMoving`))
    (:`OnFail`
      (`self.UpdateMoving`))))

(fn `UserConstructionScript`)