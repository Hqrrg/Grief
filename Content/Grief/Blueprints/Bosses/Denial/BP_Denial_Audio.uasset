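; BP_Denial_Audio is a Denial boss Blueprint that plays location-based sounds for the boss's key combat events.
; On BeginPlay it writes player pawn 0 and a chase flag to the AI blackboard, then binds to player sensing.
; Sounds fire at the actor's location on player detection, on LaserBarrage, Hyperbeam or Slam attack starts, and on damage, with separate branches for surviving hits and zero health.
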(event `self.ReceiveBeginPlay`
  (bind _output_get (set `self.BlackboardRef` (`AIBlueprintHelperLibrary.GetBlackboard` (`AIBlueprintHelperLibrary.GetAIController` self))))
  (`BlackboardComponent.SetValueAsObject` _output_get (`self.BlackboardPlayerKey`) (`GameplayStatics.GetPlayerPawn` 0))
  (`BlackboardComponent.SetValueAsBool` (`self.BlackboardRef`) (`self.BlackboardShouldChaseKey`) true)
  (add `PlayerSensingComponent.OnPlayerSensed` (`self.PlayerSensing`) (delegate `Sensed`)))

(event `Sensed`
  (params (Player :type "PlayerPawn Object Reference") (Detected :type Boolean) (SensingRange :type "ESensingRange Enum" :default "None") (HasLineOfSight :type Boolean))
  (if Detected
    (`GameplayStatics.PlaySoundAtLocation` null (`self.K2_GetActorLocation`) (struct) 1.0 1.0 0.0 null null null null)))

(event `self.OnBeginAttack`
  (params (AttackID :type Byte))
  (if (== AttackID (`self.GetAttackID` "LaserBarrage"))
    (`GameplayStatics.PlaySoundAtLocation` null (`self.K2_GetActorLocation`) (struct) 1.0 1.0 0.0 null null null null)
    (elif (== AttackID (`self.GetAttackID` "Hyperbeam"))
      (`GameplayStatics.PlaySoundAtLocation` null (`self.K2_GetActorLocation`) (struct) 1.0 1.0 0.0 null null null null)
      (elif (== AttackID (`self.GetAttackID` "Slam"))
        (`GameplayStatics.PlaySoundAtLocation` null (`self.K2_GetActorLocation`) (struct) 1.0 1.0 0.0 null null null null)))))

(event `self.OnTakeDamage`
  (params (NewHealth :type "Float (single-precision)"))
  (bind _returnvalue (`self.K2_GetActorLocation`))
  (if (> NewHealth 0.0)
    (`GameplayStatics.PlaySoundAtLocation` null _returnvalue (struct) 1.0 1.0 0.0 null null null null)
    (else
      (`GameplayStatics.PlaySoundAtLocation` null _returnvalue (struct) 1.0 1.0 0.0 null null null null))))

(fn `UserConstructionScript`)