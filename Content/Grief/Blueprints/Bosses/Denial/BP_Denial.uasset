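; BP_Denial is the Denial boss, whose blueprint links player sensing to its AI, health bar UI and sound cues.
; Sensing the player writes the target and start flag to the AI Blackboard and shows a boss bar while alive; escape clears the flag and removes the bar.
; Damage plays sounds, and zero health removes top-level boss bars, setting Dead inside that loop.
; LaserBarrage, Hyperbeam and Slam attacks trigger sounds as they begin.
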(event `self.ReceiveBeginPlay`
  (set `self.BlackboardRef` (`AIBlueprintHelperLibrary.GetBlackboard` (`AIBlueprintHelperLibrary.GetAIController` self))))

(event `self.PlayerSensing.OnPlayerSensed`
  (params (Player :type "PlayerPawn Object Reference") (Detected :type Boolean) (SensingRange :type "ESensingRange Enum" :default "None") (HasLineOfSight :type Boolean))
  (if Detected
    (`BlackboardComponent.SetValueAsObject` (`self.BlackboardRef`) (`self.BlackboardPlayerKey`) Player)
    (`BlackboardComponent.SetValueAsBool` (`self.BlackboardRef`) (`self.BlackboardStart`) true)
    (if (not (`self.Dead`))
      (bind _returnvalue (`|CreateWidget` "/Game/Grief/Blueprints/UI/DenialBossBar.DenialBossBar_C"))
      (bind _output_get (set `self.Widget` _returnvalue))
      (`UserWidget.AddToViewport` _output_get 0))
    (if true
      (`GameplayStatics.PlaySoundAtLocation` null (`self.K2_GetActorLocation`) (struct) 1.0 1.0 0.0 null null null null))))

(event `self.PlayerSensing.OnPlayerEscaped`
  (params (Player :type "PlayerPawn Object Reference"))
  (`BlackboardComponent.SetValueAsBool` (`self.BlackboardRef`) (`self.BlackboardStart`) false)
  (`Widget.RemoveFromParent` (`self.Widget`)))

(event `self.OnTakeDamage`
  (params (NewHealth :type "Float (single-precision)"))
  (bind _returnvalue (`self.K2_GetActorLocation`))
  (bind _output_get (set `self.Boss New Health` NewHealth))
  (if (> _output_get 0.0)
    (`GameplayStatics.PlaySoundAtLocation` null _returnvalue (struct) 1.0 1.0 0.0 null null null null)
    (else
      (`GameplayStatics.PlaySoundAtLocation` null _returnvalue (struct) 1.0 1.0 0.0 null null null null)))
  (if (== (`self.Boss New Health`) 0.0)
    (bind _foundwidgets (`WidgetBlueprintLibrary.GetAllWidgetsOfClass` "/Game/Grief/Blueprints/UI/DenialBossBar.DenialBossBar_C"))
    (for _array_element _foundwidgets
      (`Widget.RemoveFromParent` _array_element)
      (set `self.Dead` true))))

(event `self.OnBeginAttack`
  (params (AttackID :type Byte))
  (if (== AttackID (`self.GetAttackID` "LaserBarrage"))
    (`GameplayStatics.PlaySoundAtLocation` null (`self.K2_GetActorLocation`) (struct) 1.0 1.0 0.0 null null null null)
    (elif (== AttackID (`self.GetAttackID` "Hyperbeam"))
      (`GameplayStatics.PlaySoundAtLocation` null (`self.K2_GetActorLocation`) (struct) 1.0 1.0 0.0 null null null null)
      (elif (== AttackID (`self.GetAttackID` "Slam"))
        (`GameplayStatics.PlaySoundAtLocation` null (`self.K2_GetActorLocation`) (struct) 1.0 1.0 0.0 null null null null)))))

(fn `UserConstructionScript`)