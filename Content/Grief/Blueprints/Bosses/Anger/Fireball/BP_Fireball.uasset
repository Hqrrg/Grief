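; BP_Fireball is a fireball Blueprint for the Anger boss, with placeholder responses to projectile lifecycle events.
; Fired, Collided and Retrieved events only print debug strings, distinguishing a hit from a miss and an expired lifetime from a recall.
; It contains no movement, damage or effect logic, and its BeginPlay, overlap, Tick and construction script are empty.
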(event `self.Fired`
  (`KismetSystemLibrary.PrintString` "Fired"))

(event `self.Collided`
  (params (HitTarget :type Boolean))
  (`KismetSystemLibrary.PrintString` (`KismetStringLibrary.Concat_StrStr` "Collided: " (select `bool` HitTarget :`false` "Missed" :`true` "Hit"))))

(event `self.Retrieved`
  (params (LifetimeElapsed :type Boolean))
  (`KismetSystemLibrary.PrintString` (`KismetStringLibrary.Concat_StrStr` "Retrieved: " (select `bool` LifetimeElapsed :`false` "Recalled" :`true` "Lifetime Elapsed"))))

(fn `UserConstructionScript`)