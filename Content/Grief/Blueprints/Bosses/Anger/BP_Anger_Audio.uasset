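; Audio Blueprint for the Anger boss, playing sounds at its location for attacks and damage.
; The attack-begin event matches the attack ID against Fireball, Beam and Outburst, with a separate sound call for each.
; The damage event branches on whether health remains above zero to separate hit from death sounds.
; BeginPlay also caches the AI blackboard and writes the player pawn to it.
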(event `self.ReceiveBeginPlay`
  (set `self.BlackboardRef` (`AIBlueprintHelperLibrary.GetBlackboard` (`AIBlueprintHelperLibrary.GetAIController` self)))
  (`BlackboardComponent.SetValueAsObject` (`self.BlackboardRef`) (`self.BlackboardPlayerKey`) (`GameplayStatics.GetPlayerPawn` 0)))

(event `self.OnBeginAttack`
  (params (AttackID :type Byte))
  (if (== AttackID (`self.GetAttackID` "Fireball"))
    (`GameplayStatics.PlaySoundAtLocation` null (`self.K2_GetActorLocation`) (struct) 1.0 1.0 0.0 null null null null)
    (elif (== AttackID (`self.GetAttackID` "Beam"))
      (`GameplayStatics.PlaySoundAtLocation` null (`self.K2_GetActorLocation`) (struct) 1.0 1.0 0.0 null null null null)
      (elif (== AttackID (`self.GetAttackID` "Outburst"))
        (`GameplayStatics.PlaySoundAtLocation` null (`self.K2_GetActorLocation`) (struct) 1.0 1.0 0.0 null null null null)))))

(event `self.OnTakeDamage`
  (params (NewHealth :type "Float (single-precision)"))
  (bind _returnvalue (`self.K2_GetActorLocation`))
  (if (> NewHealth 0.0)
    (`GameplayStatics.PlaySoundAtLocation` null _returnvalue (struct) 1.0 1.0 0.0 null null null null)
    (else
      (`GameplayStatics.PlaySoundAtLocation` null _returnvalue (struct) 1.0 1.0 0.0 null null null null))))

(fn `UserConstructionScript`)