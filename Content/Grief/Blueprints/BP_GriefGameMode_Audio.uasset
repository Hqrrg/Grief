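; BP_GriefGameMode_Audio runs the looping background ambience for Grief, alternating between a forest rain track and a night forest track.
; BeginPlay starts the rain and two looping timers of equal period, offset by a negative initial delay so night plays for the last quarter of each cycle.
; Each timer event crossfades by fading out the current component and fading in a newly created 2D sound.
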(event `self.ReceiveBeginPlay`
  (bind _returnvalue (`GameplayStatics.SpawnSound2D` "/Game/Grief/Audio/forest-rain-atmo-fantasy-14435.forest-rain-atmo-fantasy-14435" 0.7 1.0 0.0 null))
  (set `self.AmbienceComponent1` _returnvalue)
  (`KismetSystemLibrary.K2_SetTimerDelegate` (delegate `FadeAmbience1`) 120.0 true -30.0)
  (`KismetSystemLibrary.K2_SetTimerDelegate` (delegate `FadeAmbience2`) 120.0 true))

(event `FadeAmbience1`
  (`AudioComponent.FadeOut` (`self.AmbienceComponent1`) 5.0 0.0 "Linear")
  (bind _returnvalue (`GameplayStatics.CreateSound2D` "/Game/Grief/Audio/mixkit-forest-at-night-1224.mixkit-forest-at-night-1224" 0.4 1.0 0.0 null))
  (bind _output_get (set `self.AmbienceComponent2` _returnvalue))
  (`AudioComponent.FadeIn` _output_get 5.0 1.0 0.0 "Linear"))

(event `FadeAmbience2`
  (`AudioComponent.FadeOut` (`self.AmbienceComponent2`) 5.0 0.0 "Linear")
  (bind _returnvalue (`GameplayStatics.CreateSound2D` "/Game/Grief/Audio/forest-rain-atmo-fantasy-14435.forest-rain-atmo-fantasy-14435" 0.5 1.0 0.0 null))
  (bind _output_get (set `self.AmbienceComponent1` _returnvalue))
  (`AudioComponent.FadeIn` _output_get 5.0 1.0 0.0 "Linear"))

(fn `UserConstructionScript`)