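; BP_EnemyCharacter is an enemy character that chases the player and attacks on reaching them.
; It caches the player character at BeginPlay, then reissues AI MoveTo toward it every Tick while not attacking.
; Each request updates facing directions from the movement vector and refreshes the moving state.
; Success refreshes that state and triggers an attack by EnemyAttackID, while failure only refreshes it.
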(event `self.ReceiveBeginPlay`
  (bind _asbp_player_character (cast `/Game/Grief/Blueprints/Player/BP_PlayerCharacter` (`GameplayStatics.GetPlayerCharacter` 0)))
  (set `self.PlayerRef` _asbp_player_character))

(event `self.ReceiveTick`
  (params (DeltaSeconds :type "Float (single-precision)"))
  (if (not (`self.IsAttacking`))
    (`|AIMoveTo` self (0.0 0.0 0.0) (`self.PlayerRef`) 100.0
      (:`then`
        (`self.UpdateDirections` (`self.GetMovementVector`))
        (`self.UpdateMoving`))
      (:`OnSuccess`
        (`self.UpdateMoving`)
        (`self.Attack` (`self.EnemyAttackID`)))
      (:`OnFail`
        (`self.UpdateMoving`)))))

(fn `UserConstructionScript`)