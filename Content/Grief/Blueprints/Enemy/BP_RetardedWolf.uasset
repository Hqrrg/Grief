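; Simple wolf enemy that paces back and forth along the world Y axis, with no target detection.
; It records its spawn location on BeginPlay, then issues an AI move request from Tick to that location plus a Y offset.
; Each successful move toggles the offset between zero and a fixed distance.
; The move outputs also refresh its moving state, and the immediate output updates facing directions from the movement vector.
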(event `self.ReceiveBeginPlay`
  (set `self.SpawnLocation` (`self.K2_GetActorLocation`)))

(event `self.ReceiveTick`
  (params (DeltaSeconds :type "Float (single-precision)"))
  (bind (_spawnlocation_x _spawnlocation_y _spawnlocation_z) (`KismetMathLibrary.BreakVector` (`self.SpawnLocation`)))
  (`AIPawnFunctionLibrary.AIPawnMoveToLocation` (`AIBlueprintHelperLibrary.GetAIController` self) (`KismetMathLibrary.MakeVector` _spawnlocation_x (+ _spawnlocation_y (`self.MoveYBias`)) _spawnlocation_z)
    (:`Out`
      (`self.UpdateDirections` (`self.GetMovementVector`))
      (`self.UpdateMoving`))
    (:`Success`
      (`self.UpdateMoving`)
      (if (> (`self.MoveYBias`) 0.0)
        (set `self.MoveYBias` 0.0)
        (else
          (set `self.MoveYBias` 500.0))))
    (:`Failure`
      (`self.UpdateMoving`))))

(fn `UserConstructionScript`)