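; BP_Player is the player character Blueprint, which here handles the player's sound effects.
; On BeginPlay it binds jump and land events from its MovementComponent, which also supplies a footstep event.
; Those movement events, attack start and damage each play a sound at the actor's location.
; Damage picks a hurt or death cue depending on whether the new health is above zero.
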(event `self.ReceiveBeginPlay`
  (bind _movementcomponent (`self.MovementComponent`))
  (add `PlatformPawnMovement.OnJumped` _movementcomponent (delegate `EventJump`))
  (add `PlatformPawnMovement.OnLanded` _movementcomponent (delegate `EventLanded`)))

(event `EventJump`
  (`GameplayStatics.PlaySoundAtLocation` "/Game/Grief/Audio/hero_jump.hero_jump" (`self.K2_GetActorLocation`) (struct) 1.0 1.0 0.0 null null null null))

(event `EventLanded`
  (`GameplayStatics.PlaySoundAtLocation` "/Game/Grief/Audio/FootstepsStoneDirt4.FootstepsStoneDirt4" (`self.K2_GetActorLocation`) (struct) 1.0 1.0 0.0 null null null null))

(event `self.MovementComponent.OnFootstep`
  (`GameplayStatics.PlaySoundAtLocation` "/Game/Grief/Audio/FootstepCue.FootstepCue" (`self.K2_GetActorLocation`) (struct) 1.0 1.0 0.0 null null null null))

(event `self.OnBeginAttack`
  (params (AttackID :type Byte))
  (`GameplayStatics.PlaySoundAtLocation` "/Game/Grief/Audio/SwordSwingCue.SwordSwingCue" (`self.K2_GetActorLocation`) (struct) 1.0 1.0 0.0 null null null null))

(event `self.OnTakeDamage`
  (params (NewHealth :type "Float (single-precision)"))
  (bind _returnvalue (`self.K2_GetActorLocation`))
  (if (> NewHealth 0.0)
    (`GameplayStatics.PlaySoundAtLocation` "/Game/Grief/Audio/HurtPlayerCue.HurtPlayerCue" _returnvalue (struct) 1.0 1.0 0.0 null null null null)
    (else
      (`GameplayStatics.PlaySoundAtLocation` "/Game/Grief/Audio/DeadPlayerCue.DeadPlayerCue" _returnvalue (struct) 1.0 1.0 0.0 null null null null))))

(fn `UserConstructionScript`)