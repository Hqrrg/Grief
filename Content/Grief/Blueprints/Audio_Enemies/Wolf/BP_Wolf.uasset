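; BP_Wolf is a wolf enemy that chases the player and plays beast sounds for its reactions.
; Player sensing events write the target and chase flag to the AI controller's blackboard, and losing the player clears the flag and stops movement immediately.
; Detection, escape, attack, hit and death each play a sound at the wolf's location, with remaining health choosing between hit and death.
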(event `self.PlayerSensing.OnPlayerSensed`
  (params (Player :type "PlayerPawn Object Reference") (Detected :type Boolean) (SensingRange :type "ESensingRange Enum" :default "None") (HasLineOfSight :type Boolean))
  (if Detected
    (`BlackboardComponent.SetValueAsObject` (`AIBlueprintHelperLibrary.GetBlackboard` (`AIBlueprintHelperLibrary.GetAIController` self)) "Player" Player)
    (`BlackboardComponent.SetValueAsBool` (`AIBlueprintHelperLibrary.GetBlackboard` (`AIBlueprintHelperLibrary.GetAIController` self)) "ShouldChase" true)
    (`GameplayStatics.PlaySoundAtLocation` "/Game/Grief/Audio/BeastSeePlayer.BeastSeePlayer" (`self.K2_GetActorLocation`) (struct) 1.0 1.0 0.0 null null null null)))

(event `self.PlayerSensing.OnPlayerEscaped`
  (params (Player :type "PlayerPawn Object Reference"))
  (`BlackboardComponent.SetValueAsBool` (`AIBlueprintHelperLibrary.GetBlackboard` (`AIBlueprintHelperLibrary.GetAIController` self)) "ShouldChase" false)
  (`MovementComponent.StopMovementImmediately` (`self.MovementComponent`))
  (`self.UpdateMoving`)
  (`GameplayStatics.PlaySoundAtLocation` "/Game/Grief/Audio/BeastLosePlayer.BeastLosePlayer" (`self.K2_GetActorLocation`) (struct) 1.0 1.0 0.0 null null null null))

(event `self.OnAttack`
  (params (AttackID :type Byte))
  (`GameplayStatics.PlaySoundAtLocation` "/Game/Grief/Audio/BeastAttack.BeastAttack" (`self.K2_GetActorLocation`) (struct) 1.0 1.0 0.0 null null null null))

(event `self.OnTakeDamage`
  (params (NewHealth :type "Float (single-precision)"))
  (bind _returnvalue (`self.K2_GetActorLocation`))
  (if (> NewHealth 0.0)
    (`GameplayStatics.PlaySoundAtLocation` "/Game/Grief/Audio/GenericHit.GenericHit" _returnvalue (struct) 1.0 1.0 0.0 null null null null)
    (else
      (`GameplayStatics.PlaySoundAtLocation` "/Game/Grief/Audio/BeastDeath.BeastDeath" _returnvalue (struct) 1.0 1.0 0.0 null null null null))))

(fn `UserConstructionScript`)